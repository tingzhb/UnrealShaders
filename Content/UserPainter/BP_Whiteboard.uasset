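; Whiteboard actor that players can paint on at runtime by drawing marker strokes into a render target.
; On BeginPlay it creates a 2048 render target, binds it to the board mesh through a dynamic material, and creates a dynamic M_Marker instance.
; DrawOnBoard passes a 2D location to the marker material and draws that material onto the render target, updating the visible board.
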(event `self.ReceiveBeginPlay`
  (bind _sm_whiteboard (`self.SM_Whiteboard`))
  (bind _returnvalue (`KismetRenderingLibrary.CreateRenderTarget2D` 2048 2048))
  (set `self.PaintBoard RT` _returnvalue)
  (bind _returnvalue_2 (`PrimitiveComponent.CreateDynamicMaterialInstance` _sm_whiteboard 0 (`PrimitiveComponent.GetMaterial` _sm_whiteboard 0) "None"))
  (`MaterialInstanceDynamic.SetTextureParameterValue` _returnvalue_2 "RT_PaintBoard" (`self.PaintBoard RT`))
  (`PrimitiveComponent.SetMaterial` _sm_whiteboard 0 _returnvalue_2)
  (bind _returnvalue_3 (`KismetMaterialLibrary.CreateDynamicMaterialInstance` "/Game/UserPainter/M_Marker.M_Marker"))
  (set `self.MarkerMID` _returnvalue_3))

(event `DrawOnBoard`
  (params (DrawLocation :type "Vector2D Structure"))
  (bind _markermid (`self.MarkerMID`))
  (`MaterialInstanceDynamic.SetVectorParameterValue` _markermid "DrawLocation" (`KismetMathLibrary.Conv_VectorToLinearColor` (`KismetMathLibrary.Conv_Vector2DToVector` DrawLocation 0.1)))
  (`KismetRenderingLibrary.DrawMaterialToRenderTarget` (`self.PaintBoard RT`) _markermid))

(fn `UserConstructionScript`)